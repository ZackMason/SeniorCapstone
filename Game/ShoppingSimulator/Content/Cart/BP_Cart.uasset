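; BP_Cart is a physics cart whose Box body is pushed upward by four corner springs, like a simple suspension.
; Each Tick it casts the four child actors to BP_CartSpring in BR, BL, FL, FR order; a failed cast skips the remaining springs.
; Each spring calculates its own strength, and positive values become impulses along the Box's up vector at that spring's location.
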(event `self.ReceiveTick`
  (params (DeltaSeconds :type "Float (single-precision)"))
  (bind _asbp_cart_spring (cast `/Game/Cart/BP_CartSpring` (`ChildActorComponent.ChildActor` (`self.BP_CartSpringBR`))))
  (`self.ApplySpringImpulse` _asbp_cart_spring)
  (bind _asbp_cart_spring_2 (cast `/Game/Cart/BP_CartSpring` (`ChildActorComponent.ChildActor` (`self.BP_CartSpringBL`))))
  (`self.ApplySpringImpulse` _asbp_cart_spring_2)
  (bind _asbp_cart_spring_3 (cast `/Game/Cart/BP_CartSpring` (`ChildActorComponent.ChildActor` (`self.BP_CartSpringFL`))))
  (`self.ApplySpringImpulse` _asbp_cart_spring_3)
  (bind _asbp_cart_spring_4 (cast `/Game/Cart/BP_CartSpring` (`ChildActorComponent.ChildActor` (`self.BP_CartSpringFR`))))
  (`self.ApplySpringImpulse` _asbp_cart_spring_4))

(fn `ApplySpringImpulse`
  (params (Spring :type "/Game/Cart/BP_CartSpring Object Reference"))
  (bind _box (`self.Box`))
  (bind _impulse (`/Game/Cart/BP_CartSpring.CalculateImpulseStrength` Spring))
  (if (> _impulse 0.0)
    (`PrimitiveComponent.AddImpulseAtLocation` _box (* (`SceneComponent.GetUpVector` _box) _impulse) (`self.K2_GetActorLocation` Spring) "None")))

(fn `UserConstructionScript`)