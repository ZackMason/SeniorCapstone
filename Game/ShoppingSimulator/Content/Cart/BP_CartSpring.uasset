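; BP_CartSpring is a cart spring Blueprint that computes a suspension-style impulse strength from a downward or offset line trace.
; CalculateImpulseStrength traces on Visibility using TargetDistance, returning the gap between TargetDistance and hit distance times SpringConstant, or zero without a hit.
; Tick runs a similar debug-drawn trace on a different axis but does nothing with the result.
; No impulse is applied within this Blueprint.
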(event `self.ReceiveTick`
  (params (DeltaSeconds :type "Float (single-precision)"))
  (bind _result (`/Engine/EditorBlueprintResources/StandardMacros.NegateFloat` (`self.TargetDistance`))
    (:`  `
      (bind _outhit (`KismetSystemLibrary.LineTraceSingle` :`End` (`KismetMathLibrary.MakeVector` 0.0 _result) :`TraceChannel` "TraceTypeQuery1" :`bTraceComplex` true :`DrawDebugType` "ForDuration"))
      (if (`GameplayStatics.BreakHitResult` _outhit)
        _))))

(fn `CalculateImpulseStrength`
  (returns (Impulse :type "Float (double-precision)"))
  (bind _result (`/Engine/EditorBlueprintResources/StandardMacros.NegateFloat` (`self.TargetDistance`))
    (:`  `
      (bind (_outhit _returnvalue) (`KismetSystemLibrary.LineTraceSingle` :`End` (`KismetMathLibrary.MakeVector` 0.0 0.0 _result) :`TraceChannel` "TraceTypeQuery1" :`bTraceComplex` true :`DrawDebugType` "Persistent"))
      (if _returnvalue
        (return (* (- (`self.TargetDistance`) (`.Distance` (`GameplayStatics.BreakHitResult` _outhit))) (`self.SpringConstant`)))
        (else
          (return 0.0))))))

(fn `UserConstructionScript`)